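; Base projectile enemy for the 2D endless runner that flies along the X axis and damages the player on contact.
; Tick moves it by speed and direction while movement is enabled, destroying it at or below an X cutoff.
; Overlapping the player's capsule sends damage to the GameMode through an interface message, then destroys the projectile.
; A GameMode max-difficulty flag adds bonus damage once before the hit is reported.
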(event OnComponentBeginOverlap(Collision)
  (params (OverlappedComponent :type Primitive%20Component%20Object%20Reference) (OtherActor :type Actor%20Object%20Reference) (OtherComp :type Primitive%20Component%20Object%20Reference) (OtherBodyIndex :type Integer) (bFromSweep :type Boolean) (SweepResult :type Hit%20Result%20Structure%20%28by%20ref%29))
  (bind _returnvalue (Game|GetPlayerCharacter 0))
  ;[1 1 1] Enemy-Player Collision
  ;;[0.4588 0.6588 1] Check if colided with player
  (Utilities|IsValid _returnvalue
    (:Is%20Valid
      (if (== OtherComp (Variables|/Script/Engine.Character|GetCapsuleComponent _returnvalue))
        ;;[0.4588 0.6588 1] Set the amount of damage done to the player
        (CallFunction|IncreaseDMG) ; Increase damage on max difficulty
        (Class|BPIGameModeCommunication|EnemyDamageInterface(Message) (Game|GetGameMode) (Variables|Damage|GetDamageAmount))
        (Actor|DestroyActor)))))

(event Custom|IncreaseDMG
  ;[1 1 1] Increased Damage on maximum diffculty
  (if (Variables|/Game/EndlessRunner2D/Blueprints/BP_GameMode.BP_GameMode_C|GetIncreaseDMG (.AsBP%20Game%20Mode (Utilities|Casting|CastToBP_GameMode (Game|GetGameMode))))
    (Utilities|FlowControl|DoOnce false
      (:Completed
        (Variables|Damage|SetDamageAmount (+ (Variables|Damage|GetDamageAmount) (Variables|Damage|GetBonusDamage)))))))

(event EventTick
  (params (DeltaSeconds :type Float%20%28single-precision%29))
  ;[1 1 1] Actor movement - set the speed and direction
  (if (Variables|Actormovement|GetCanMove)
    (Transformation|AddActorWorldOffset (Math|Vector|MakeVector (* (Variables|ActorMovement|GetSpeed) (Variables|ActorMovement|GetDirection) DeltaSeconds) 0.0 0.0))
    ;[1 1 1] Set the maximum coordinates at which the actor gets destroyed
    (if (<= (.x (Transformation|GetActorLocation)) (Variables|ActorMovement|GetDestroyCoordinates))
      (Actor|DestroyActor))))

(fn ConstructionScript)