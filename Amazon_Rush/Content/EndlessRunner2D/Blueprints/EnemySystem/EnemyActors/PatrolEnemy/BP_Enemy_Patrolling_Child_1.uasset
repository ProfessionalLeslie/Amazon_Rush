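; Child patrolling enemy for the 2D endless runner that moves its Body through three target points in a loop.
; While CanPatrol is set, Tick calls Patrol, which interpolates Body's relative location toward the current target with VInterpTo.
; On arriving within a small tolerance, it waits TargetDelay, then advances the NextTarget index, resetting to the first after the third.
; More waypoints require adding cases to the switch.
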(event Custom|Patrol
  (Utilities|IsValid (Variables|Default|GetBody)
    (:Is%20Valid
      (switch int (Variables|PatrolState|GetNextTarget) ; Add pins for more Next Targets
        (:0
          ;[1 1 1] Send the spawn point to each target
          ;;[0.4588 0.6588 1] Actor movement to target
          (Transformation|SetRelativeLocation (Variables|Default|GetBody) (Math|Interpolation|VInterpTo (Variables|/Script/Engine.SceneComponent|GetRelativeLocation (Variables|Default|GetBody)) (Variables|PatrolCoordinates|GetTarget1) (Utilities|Time|GetWorldDeltaSeconds) (Variables|PatrolState|GetInterpolation%20speed)) false false)
          ;;[0.4588 0.6588 1] Go to the next target
          (if (Math|Vector|Equal(Vector) (Variables|/Script/Engine.SceneComponent|GetRelativeLocation (Variables|Default|GetBody)) (Variables|PatrolCoordinates|GetTarget1) 1.0)
            (Utilities|FlowControl|Delay (Variables|PatrolState|GetTargetDelay))
            ;;[0.4588 0.6588 1] Iterate through the targets
            (Variables|PatrolState|SetNextTarget (+ (Variables|PatrolState|GetNextTarget) 1))))
        (:1
          (Transformation|SetRelativeLocation (Variables|Default|GetBody) (Math|Interpolation|VInterpTo (Variables|/Script/Engine.SceneComponent|GetRelativeLocation (Variables|Default|GetBody)) (Variables|PatrolCoordinates|GetTarget2) (Utilities|Time|GetWorldDeltaSeconds) (Variables|PatrolState|GetInterpolation%20speed)) false false)
          (if (Math|Vector|Equal(Vector) (Variables|/Script/Engine.SceneComponent|GetRelativeLocation (Variables|Default|GetBody)) (Variables|PatrolCoordinates|GetTarget2) 1.0)
            (Utilities|FlowControl|Delay (Variables|PatrolState|GetTargetDelay))
            (Variables|PatrolState|SetNextTarget (+ (Variables|PatrolState|GetNextTarget) 1))))
        (:2
          (Transformation|SetRelativeLocation (Variables|Default|GetBody) (Math|Interpolation|VInterpTo (Variables|/Script/Engine.SceneComponent|GetRelativeLocation (Variables|Default|GetBody)) (Variables|PatrolCoordinates|GetTarget3) (Utilities|Time|GetWorldDeltaSeconds) (Variables|PatrolState|GetInterpolation%20speed)) false false)
          (if (Math|Vector|Equal(Vector) (Variables|/Script/Engine.SceneComponent|GetRelativeLocation (Variables|Default|GetBody)) (Variables|PatrolCoordinates|GetTarget3) 1.0)
            (Utilities|FlowControl|Delay (Variables|PatrolState|GetTargetDelay))
            ;;;[1 0.08333 0.08333] Reset to 1st target
            (Variables|PatrolState|SetNextTarget 0) ; Set to 0 to go to the first target
          ))))))

(event EventTick
  (params (DeltaSeconds :type Float%20%28single-precision%29))
  (|CallParentFunction DeltaSeconds)
  (if (Variables|PatrolState|GetCanPatrol)
    (CallFunction|Patrol) ; Start the patrol event
  ))

(fn ConstructionScript
  (|CallParentFunction))