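; Main patrolling enemy for the 2D endless runner, moving along X and destroying itself past a coordinate limit.
; Player contact sends damage to the GameMode, with a one-time bonus when its IncreaseDMG flag is set.
; A falling player high enough above the death trigger kills it, getting launched upward with sound and particles.
; Tick caches player height for that stomp check while CanBeKilled is set.
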(event OnComponentBeginOverlap(DeathTrigger)
  (params (OverlappedComponent :type Primitive%20Component%20Object%20Reference) (OtherActor :type Actor%20Object%20Reference) (OtherComp :type Primitive%20Component%20Object%20Reference) (OtherBodyIndex :type Integer) (bFromSweep :type Boolean) (SweepResult :type Hit%20Result%20Structure%20%28by%20ref%29))
  (bind _returnvalue (Game|GetPlayerCharacter 0))
  ;[1 1 1] Death trigger <=> Player colision check
  ;;[0.4588 0.6588 1] Check if colided with player
  (if (== OtherComp (Variables|/Script/Engine.Character|GetCapsuleComponent (Game|GetPlayerCharacter 0)))
    (if (and (< (+ (.z (Transformation|GetWorldLocation (Variables|Default|GetDeathTrigger))) (Variables|/Script/Engine.CapsuleComponent|GetCapsuleHalfHeight (Variables|/Script/Engine.Character|GetCapsuleComponent _returnvalue))) (stale Custom|KillActor _output_get)) (AI|Components|NavMovement|IsFalling (Variables|/Script/Engine.Character|GetCharacterMovement _returnvalue)))
      ;;[0.4588 0.6588 1] Disable the default collision
      (Collision|SetCollisionEnabled (Variables|Default|GetCollision) "NoCollision")
      ;;[0.4588 0.6588 1] Player mini jump on enemy death
      (Character|LaunchCharacter (Game|GetPlayerCharacter 0) "0, 0,500.000000" true true) ; On kill sends the player upwards
      (Audio|PlaySound2D "/Game/EndlessRunner2D/SFX/Gameplay/Cue/SC_EnemyDeath.SC_EnemyDeath")
      ;;[0.4588 0.6588 1] Spawn the hit effect
      (Effects|SpawnEmitteratLocation "/Game/EndlessRunner2D/GFX/Particles/EnemyDie/PS_EnemyDestroy.PS_EnemyDestroy" (Transformation|GetWorldLocation (Variables|Default|GetBody)))
      (Actor|DestroyActor))))

(event OnComponentBeginOverlap(Collision)
  (params (OverlappedComponent :type Primitive%20Component%20Object%20Reference) (OtherActor :type Actor%20Object%20Reference) (OtherComp :type Primitive%20Component%20Object%20Reference) (OtherBodyIndex :type Integer) (bFromSweep :type Boolean) (SweepResult :type Hit%20Result%20Structure%20%28by%20ref%29))
  (bind _returnvalue (Game|GetPlayerCharacter 0))
  ;[1 1 1] Enemy-Player Collision
  ;;[0.4588 0.6588 1] Check if colided with player
  (Utilities|IsValid _returnvalue
    (:Is%20Valid
      (if (== OtherComp (Variables|/Script/Engine.Character|GetCapsuleComponent _returnvalue))
        ;;[0.4588 0.6588 1] Set the amount of damage done to the player
        (CallFunction|IncreaseDMG) ; Increase damage on max difficulty
        (Class|BPIGameModeCommunication|EnemyDamageInterface(Message) (Game|GetGameMode) (Variables|Damage|GetDamageAmount))
        (Actor|DestroyActor)))))

(event Custom|KillActor
  (bind _returnvalue (Game|GetPlayerCharacter 0))
  ;[1 1 1] Death trigger event - check character height
  (if (Variables|KillTrigger|GetCanBeKilled)
    (Utilities|IsValid _returnvalue
      (:Is%20Valid
        ;;[0.4588 0.6588 1] Kill condition = player > player/2 + death trigger (coord)
        (bind _output_get (Variables|KillTrigger|SetPlayerLocation_Z (.z (Transformation|GetWorldLocation (Variables|/Script/Engine.Character|GetCapsuleComponent _returnvalue)))))))))

(event Custom|IncreaseDMG
  ;[1 1 1] Increased Damage on maximum diffculty
  (if (Variables|/Game/EndlessRunner2D/Blueprints/BP_GameMode.BP_GameMode_C|GetIncreaseDMG (.AsBP%20Game%20Mode (Utilities|Casting|CastToBP_GameMode (Game|GetGameMode))))
    (Utilities|FlowControl|DoOnce false
      (:Completed
        (Variables|Damage|SetDamageAmount (+ (Variables|Damage|GetDamageAmount) (Variables|Damage|GetBonusDamage)))))))

(event EventTick
  (params (DeltaSeconds :type Float%20%28single-precision%29))
  (CallFunction|KillActor) ; Calls the enemy death event
  ;[1 1 1] Actor movement - set the speed and direction
  (if (Variables|Actormovement|GetCanMove)
    (Transformation|AddActorWorldOffset (Math|Vector|MakeVector (* (Variables|Actormovement|GetSpeed) (Variables|Actormovement|GetDirection) DeltaSeconds) 0.0 0.0))
    ;[1 1 1] Set the maximum coordinates at which the actor gets destroyed
    (if (<= (.x (Transformation|GetActorLocation)) (Variables|Actormovement|GetDestroyCoordinates))
      (Actor|DestroyActor))))

(fn ConstructionScript)