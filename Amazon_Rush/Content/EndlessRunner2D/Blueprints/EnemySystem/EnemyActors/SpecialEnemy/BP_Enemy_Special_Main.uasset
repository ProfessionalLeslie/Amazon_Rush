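; Special enemy for the 2D endless runner that moves along X and randomly either flies past or dives at the player.
; An attacker stops at a randomly picked X threshold, flashes red, then homes on the player's saved position and self-destructs there.
; Body contact sends damage through a GameMode interface.
; A falling stomp on DeathTrigger kills it and bounces the player; that overlap also applies max-difficulty bonus damage once.
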(event OnComponentBeginOverlap(DeathTrigger)
  (params (OverlappedComponent :type Primitive%20Component%20Object%20Reference) (OtherActor :type Actor%20Object%20Reference) (OtherComp :type Primitive%20Component%20Object%20Reference) (OtherBodyIndex :type Integer) (bFromSweep :type Boolean) (SweepResult :type Hit%20Result%20Structure%20%28by%20ref%29))
  (bind _returnvalue (Game|GetPlayerCharacter 0))
  ;[1 1 1] Death trigger <=> Player colision check
  (if (== OtherComp (Variables|/Script/Engine.Character|GetCapsuleComponent (Game|GetPlayerCharacter 0)))
    (CallFunction|IncreaseDMG) ; Increase damage on max difficulty
    ;;[0.4588 0.6588 1] Disable the default collision
    (if (and (< (+ (.z (Transformation|GetWorldLocation (Variables|Default|GetDeathTrigger))) (Variables|/Script/Engine.CapsuleComponent|GetCapsuleHalfHeight (Variables|/Script/Engine.Character|GetCapsuleComponent _returnvalue))) (stale Custom|KillActor _output_get)) (AI|Components|NavMovement|IsFalling (Variables|/Script/Engine.Character|GetCharacterMovement _returnvalue)))
      (Collision|SetCollisionEnabled (Variables|Default|GetCollision) "NoCollision")
      ;;[0.4588 0.6588 1] Player mini jump on enemy death
      (Character|LaunchCharacter (Game|GetPlayerCharacter 0) "0, 0,500.000000" true true) ; On kill sends the player upwards
      ;;[0.4588 0.6588 1] Spawn the hit effect
      (Effects|SpawnEmitteratLocation "/Game/EndlessRunner2D/GFX/Particles/EnemyDie/PS_EnemyDestroy.PS_EnemyDestroy" (Transformation|GetWorldLocation (Variables|Default|GetPaperFlipbook)))
      (Audio|PlaySound2D "/Game/EndlessRunner2D/SFX/Gameplay/Cue/SC_EnemyDeath.SC_EnemyDeath")
      (Actor|DestroyActor))))

(event OnComponentBeginOverlap(Collision)
  (params (OverlappedComponent :type Primitive%20Component%20Object%20Reference) (OtherActor :type Actor%20Object%20Reference) (OtherComp :type Primitive%20Component%20Object%20Reference) (OtherBodyIndex :type Integer) (bFromSweep :type Boolean) (SweepResult :type Hit%20Result%20Structure%20%28by%20ref%29))
  (bind _returnvalue (Game|GetPlayerCharacter 0))
  ;[1 1 1] Enemy-Player Collision
  ;;[0.4588 0.6588 1] Check if colided with player
  (Utilities|IsValid _returnvalue
    (:Is%20Valid
      (if (== OtherComp (Variables|/Script/Engine.Character|GetCapsuleComponent _returnvalue))
        ;;[0.4588 0.6588 1] Set the amount of damage done to the player
        (Class|BPIGameModeCommunication|EnemyDamageInterface(Message) (Game|GetGameMode) (Variables|Damage|GetDamageAmount))
        (Actor|DestroyActor)))))

(event Custom|EnemyAttack
  ;[1 1 1] Attack event
  ;;[0.4588 0.6588 1] The actor attacks the last known player position at a certain speed
  (Transformation|SetRelativeLocation (Variables|Default|GetRoot) (Math|Interpolation|VInterptoConstant (Transformation|GetActorLocation) (Variables|Attack|GetPlayerLocation) (Utilities|Time|GetWorldDeltaSeconds) (Variables|Attack|GetAttackSpeed)) false false)
  ;;[0.4588 0.6588 1] Destroy the actor when it reaches the targeted position
  (if (Math|Vector|Equal(Vector) (Transformation|GetActorLocation) (Variables|Attack|GetPlayerLocation) 5.0)
    (Audio|PlaySound2D "/Game/EndlessRunner2D/SFX/Gameplay/Cue/SC_EnemyDeath.SC_EnemyDeath")
    (Actor|DestroyActor)))

(event Custom|KillActor
  (bind _returnvalue (Game|GetPlayerCharacter 0))
  ;[1 1 1] Death trigger event - check character height
  (if (Variables|KillTrigger|GetCanBeKilled)
    ;;[0.4588 0.6588 1] Kill condition = player > player/2 + death trigger (coord)
    (Utilities|IsValid _returnvalue
      (:Is%20Valid
        (bind _output_get (Variables|KillTrigger|SetPlayerLocation_Z (.z (Transformation|GetWorldLocation (Variables|/Script/Engine.Character|GetCapsuleComponent _returnvalue)))))))))

(event Custom|AttackHint
  (bind _paperflipbook (Variables|Default|GetPaperFlipbook))
  ;[1 1 1] Indicator that the actor is attacking
  (Audio|PlaySound2D "/Game/EndlessRunner2D/SFX/Gameplay/Cue/SC_EnemyAttack.SC_EnemyAttack")
  ;;[0.4588 0.6588 1] Attack alert > change color + animation rate + effect
  (Sprite|SetSpriteColor _paperflipbook "(R=1.000000,G=0.005000,B=0.005000,A=1.000000)")
  (Components|Timeline|SetPlayRate _paperflipbook 1e+02)
  (Components|Activation|Activate (Variables|Default|GetSawBlade_Attack) false))

(event Custom|IncreaseDMG
  ;[1 1 1] Increased Damage on maximum diffculty
  (if (Variables|/Game/EndlessRunner2D/Blueprints/BP_GameMode.BP_GameMode_C|GetIncreaseDMG (.AsBP%20Game%20Mode (Utilities|Casting|CastToBP_GameMode (Game|GetGameMode))))
    (Utilities|FlowControl|DoOnce false
      (:Completed
        (Variables|Damage|SetDamageAmount (+ (Variables|Damage|GetDamageAmount) (Variables|Damage|GetBonusDamage)))))))

(event EventTick
  (params (DeltaSeconds :type Float%20%28single-precision%29))
  (bind _returnvalue (Game|GetPlayerCharacter 0))
  (bind _attackcoordinate (Variables|Attack|GetAttackCoordinate))
  ;[1 1 1] Actor movement - set the speed and direction
  (CallFunction|KillActor) ; Trigger the kill actor event
  (if (Variables|Actormovement|GetCanMove)
    (Transformation|AddActorWorldOffset (Math|Vector|MakeVector (* (Variables|ActorMovement|GetSpeed) (Variables|ActorMovement|GetDirection) DeltaSeconds) 0.0 0.0))
    ;[1 1 1] Set the maximum coordinates at which the actor gets destroyed
    (if (<= (.x (Transformation|GetActorLocation)) (Variables|ActorMovement|GetDestroyCoordinates))
      (Actor|DestroyActor)
      (else
        ;[1 1 1] Attack event conditions if the actor has not reached its death coordinates
        ;;[0.4588 0.6588 1] Set and choose random coordinates at which to start attacking
        (if (and (<= (.x (Transformation|GetActorLocation)) (Utilities|Array|Get(acopy) _attackcoordinate (Math|Random|RandomInteger (Utilities|Array|Length _attackcoordinate)))) (Variables|Attack|GetCanAttack))
          (Variables|Actormovement|SetCanMove false) ; Starts the attack
          ;;[0.4588 0.6588 1] Get the current player position and sets as target
          (Utilities|IsValid _returnvalue
            (:Is%20Valid
              (Variables|Attack|SetPlayerLocation (Transformation|GetActorLocation _returnvalue)))))))
    (else
      ;;[0.4588 0.6588 1] Trigger the attack and attack hint
      (CallFunction|EnemyAttack)
      (Utilities|FlowControl|DoOnce false
        (:Completed
          (CallFunction|AttackHint))))))

(event EventBeginPlay
  ;[1 1 1] Toggle if this object flies by or attacks
  (Variables|Attack|SetCanAttack (Math|Random|RandomBool)))

(fn ConstructionScript)