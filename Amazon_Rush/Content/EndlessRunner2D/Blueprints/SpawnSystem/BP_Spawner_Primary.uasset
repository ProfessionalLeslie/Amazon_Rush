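; Primary spawner for the endless runner that spawns groups (holders) of rewards and patrol, simple or combo enemies at the RewardSpawning point.
; Once the game starts, Tick binds to a BP_GameMode dispatcher and spawns one reward to kick off the chain.
; Each dispatcher call rolls weighted percentages, failing with a printed error unless they total 100, then spawns a random class from the chosen category's array.
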(event Custom|SpawnTheNextObject
  (bind _patrolingenemyspawnchance (Variables|ObjectSpawnChances|GetPatrolingEnemySpawnChance))
  (bind _simpleenemyspawnchance (Variables|ObjectSpawnChances|GetSimpleEnemySpawnChance))
  (bind _rewardspawnchance (Variables|ObjectSpawnChances|GetRewardSpawnChance))
  ;[1 1 1] Primary Spawner > mainly handles spawning actor types in groups (Holders)
  ;;[0.4588 0.6588 1] Catches the event dispatcher event fom BP_GameMode when a spawned group reaches a certain coordinate triggering the next spawn
  (if (!= (+ (Variables|ObjectSpawnChances|GetPatrolingEnemySpawnChance) (Variables|ObjectSpawnChances|GetSimpleEnemySpawnChance) (Variables|ObjectSpawnChances|GetRewardSpawnChance) (Variables|ObjectSpawnChances|GetComboEnemySpawnChance)) 100) ; Fail-safe
    ;;[0.1333 0.4549 1] Spawned actors total percent value (100%) failsave
    (Development|PrintString "Spawning was intrerupting because the spawn chances sum is not 100% !!!!!!!!!!!!" true true "(R=1.000000,G=0.000000,B=0.008603,A=1.000000)" 6e+01) ; Failsafe Error
    (else
      ;[1 1 1] Percentage Chance to spawn individual actor types (ex: 60% spawn x | 30% spawn y | 10% spawn z)
      (Variables|ObjectSpawnChances|SetSpawnValuePicker (Math|Random|RandomIntegerinRange 1 100))
      (if (<= (Variables|ObjectSpawnChances|GetSpawnValuePicker) _patrolingenemyspawnchance)
        ;;[0.4588 0.6588 1] Call the functions responsible for spawning actor types
        (CallFunction|PatrolEnemySpawner) ; If the spawner has no objects to spawn, replace/delete this event
        (elif (and (> (Variables|ObjectSpawnChances|GetSpawnValuePicker) _patrolingenemyspawnchance) (<= (Variables|ObjectSpawnChances|GetSpawnValuePicker) (+ _patrolingenemyspawnchance _simpleenemyspawnchance)))
          (CallFunction|SimplePatrolSpawner) ; If the spawner has no objects to spawn, replace/delete this event
          (elif (and (> (Variables|ObjectSpawnChances|GetSpawnValuePicker) (+ _patrolingenemyspawnchance _simpleenemyspawnchance)) (<= (Variables|ObjectSpawnChances|GetSpawnValuePicker) (+ _patrolingenemyspawnchance _simpleenemyspawnchance _rewardspawnchance)))
            (CallFunction|RewardSpawner) ; If the spawner has no objects to spawn, replace/delete this event
            (elif (and (> (Variables|ObjectSpawnChances|GetSpawnValuePicker) (+ _patrolingenemyspawnchance _simpleenemyspawnchance _rewardspawnchance)) (<= (Variables|ObjectSpawnChances|GetSpawnValuePicker) (+ _patrolingenemyspawnchance _simpleenemyspawnchance _rewardspawnchance (Variables|ObjectSpawnChances|GetComboEnemySpawnChance))))
              (CallFunction|ComboEnemySpawner) ; If the spawner has no objects to spawn, replace/delete this event
            )))))))

(event EventTick
  (params (DeltaSeconds :type Float%20%28single-precision%29))
  (if (Variables|ObjectsSpawned|GetHasGameStarted?)
    ;[1 1 1] Primary Spawner > mainly handles spawning actor types in groups (Holders)
    ;;[0.4588 0.6588 1] Catches the event dispatcher event fom BP_GameMode when a spawned group reaches a certain coordinate triggering the next spawn
    (Utilities|FlowControl|Sequence
      (:then_0
        (EventDispatchers|AssignSpawnedObject<>SpawningPointPrimary (.AsBP%20Game%20Mode (Utilities|Casting|CastToBP_GameMode (Game|GetGameMode))) (delegate Custom|SpawnTheNextObject)))
      (:then_1
        ;[1 0.3798 0.4596] First spawn when the game starts > triggers the entire spawning system
        (Utilities|FlowControl|DoOnce false
          (:Completed
            (CallFunction|RewardSpawner)))))))

(fn ConstructionScript)

(fn RewardSpawner
  (bind _availablerewards (Variables|Objectsspawned|Rewards|GetAvailableRewards))
  ;[1 1 1] Rewards Spawner > spawn random elements from an array
  (Game|SpawnActorfromClass (Utilities|Array|Get(acopy) _availablerewards (Math|Random|RandomInteger (Utilities|Array|Length _availablerewards))) (Math|Transform|MakeTransform (Transformation|GetWorldLocation (Variables|Default|GetRewardSpawning)) "0, 0, 0" "1,1,1") "Undefined" 0 0))

(fn SimplePatrolSpawner
  (bind _availablesimpleenemies (Variables|Objectsspawned|Enemies|GetAvailableSimpleEnemies))
  ;[1 1 1] Simple Enemy Spawner
  (Game|SpawnActorfromClass (Utilities|Array|Get(acopy) _availablesimpleenemies (Math|Random|RandomInteger (Utilities|Array|Length _availablesimpleenemies))) (Math|Transform|MakeTransform (Transformation|GetWorldLocation (Variables|Default|GetRewardSpawning)) "0, 0, 0" "1,1,1") "Undefined" 0 0))

(fn PatrolEnemySpawner
  (bind _availablepatrolenemies (Variables|ObjectsSpawned|Enemies|GetAvailablePatrolEnemies))
  ;[1 1 1] Patrol Enemy Spawner
  (Game|SpawnActorfromClass (Utilities|Array|Get(acopy) _availablepatrolenemies (Math|Random|RandomInteger (Utilities|Array|Length _availablepatrolenemies))) (Math|Transform|MakeTransform (Transformation|GetWorldLocation (Variables|Default|GetRewardSpawning)) "0, 0, 0" "1,1,1") "Undefined" 0 0))

(fn ComboEnemySpawner
  (bind _availablecomboenemies (Variables|ObjectsSpawned|Enemies|GetAvailableComboEnemies))
  ;[1 1 1] Combo Enemy Spawner > spawn random elements from an array
  (Game|SpawnActorfromClass (Utilities|Array|Get(acopy) _availablecomboenemies (Math|Random|RandomInteger (Utilities|Array|Length _availablecomboenemies))) (Math|Transform|MakeTransform (Transformation|GetWorldLocation (Variables|Default|GetRewardSpawning)) "0, 0, 0" "1,1,1") "Undefined" 0 0))