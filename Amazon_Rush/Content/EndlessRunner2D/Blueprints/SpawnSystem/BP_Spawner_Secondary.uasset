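; Secondary spawner for the 2D endless runner that occasionally spawns a single special enemy, projectile enemy or powerup.
; It binds on Tick to the BP_GameMode dispatcher fired when a primary-spawned group reaches a set coordinate.
; Each event checks that type chances total 100%, rolls the trigger chance, then picks a type by cumulative weight.
; Per-type functions spawn a random class at RewardSpawning, optionally randomizing height from preset coordinates.
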(event Custom|SpawnTheNextSecondaryObject
  (bind _specialenemyspawnchance (Variables|ObjectSpawnChances|GetSpecialEnemySpawnChance))
  (bind _projectileenemyspawnchance (Variables|ObjectSpawnChances|GetProjectileEnemySpawnChance))
  ;[1 1 1] Secondary Spawner > mainly handles individual actor types (special enemies + powerups)
  ;;[0.4588 0.6588 1] Catches the event dispatcher event fom BP_GameMode when a spawned group from the primary spawn ponit reaches a certain coordinate and has a (%) chance to trigger this spawn point
  (if (!= (+ (Variables|ObjectSpawnChances|GetSpecialEnemySpawnChance) (Variables|ObjectSpawnChances|GetProjectileEnemySpawnChance) (Variables|ObjectSpawnChances|GetPowerUpSpawnChance)) 100) ; Fail-safe
    ;;[0.1333 0.4549 1] Spawned actors total percent value (100%) failsave
    (Development|PrintString "Spawning was intrerupting because the spawn chances sum is not 100%" true true "(R=1.000000,G=0.000000,B=0.008603,A=1.000000)" 1e+01) ; FailSafe error
    (else
      ;[1 1 1] Determine the chance to active this spawn point
      (if (<= (Math|Random|RandomIntegerinRange 1 100) (Variables|ObjectSpawnChances|GetSecondarySpawnTrigger))
        ;[1 1 1] Percentage Chance to spawn x,y,z - System
        (Variables|ObjectSpawnChances|SetSpawnValuePicker (Math|Random|RandomIntegerinRange 1 100))
        (if (<= (Variables|ObjectSpawnChances|GetSpawnValuePicker) _specialenemyspawnchance)
          ;;[0.4588 0.6588 1] Call the functions responsible for spawning actor types
          (CallFunction|SpecialEnemySpawner) ; If the spawner has no objects to spawn, replace/delete this event
          (elif (and (> (Variables|ObjectSpawnChances|GetSpawnValuePicker) _specialenemyspawnchance) (<= (Variables|ObjectSpawnChances|GetSpawnValuePicker) (+ _specialenemyspawnchance _projectileenemyspawnchance)))
            (CallFunction|ProjectileEnemySpawner) ; If the spawner has no objects to spawn, replace/delete this event
            (elif (and (> (Variables|ObjectSpawnChances|GetSpawnValuePicker) (+ _specialenemyspawnchance _projectileenemyspawnchance)) (<= (Variables|ObjectSpawnChances|GetSpawnValuePicker) (+ _specialenemyspawnchance _projectileenemyspawnchance (Variables|ObjectSpawnChances|GetPowerUpSpawnChance))))
              (CallFunction|PowerupSpawner) ; If the spawner has no objects to spawn, replace/delete this event
            )))))))

(event EventTick
  (params (DeltaSeconds :type Float%20%28single-precision%29))
  ;[1 1 1] Secondary Spawner > mainly handles individual actor types (special enemies + powerups)
  ;;[0.4588 0.6588 1] Catches the event dispatcher event fom BP_GameMode when a spawned group from the primary spawn ponit reaches a certain coordinate and has a (%) chance to trigger this spawn point
  (EventDispatchers|BindEventtoSpawnedObject<>SpawningPointSecondary (.AsBP%20Game%20Mode (Utilities|Casting|CastToBP_GameMode (Game|GetGameMode))) (delegate Custom|SpawnTheNextSecondaryObject)))

(fn ConstructionScript)

(fn PowerupSpawner
  (bind _availablepowerups (Variables|ObjectsSpawned|PowerUps|GetAvailablePowerups))
  (bind _spawncoordinate__z_axis_ (Variables|ActorSpawnPosition|GetSpawnCoordinate%20%28Z%20axis%29))
  ;[1 1 1] Powerup Spawner
  (bind _returnvalue (Game|SpawnActorfromClass (Utilities|Array|Get(acopy) _availablepowerups (Math|Random|RandomInteger (Utilities|Array|Length _availablepowerups))) (Math|Transform|MakeTransform (Transformation|GetWorldLocation (Variables|Default|GetRewardSpawning)) "0, 0,0.000000" "1,1,1") "Undefined" 0 0))
  ;[1 1 1] Set actor starting position
  (if (Variables|ActorSpawnPosition|GetRandomLocation%20%28Z%20axis%29)
    ;;[0.4588 0.6588 1] Spawn the actor randomly from an array of set coordinates
    (Transformation|SetRelativeLocation (Variables|/Game/EndlessRunner2D/Blueprints/PickupSystem/PowerUps/PowerUpActors/BP_PowerUp_Main.BP_PowerUp_Main_C|GetRoot _returnvalue) (Math|Vector|MakeVector (.x (Transformation|GetActorLocation _returnvalue)) (.y (Transformation|GetActorLocation _returnvalue)) (.z (Utilities|Array|Get(acopy) _spawncoordinate__z_axis_ (Math|Random|RandomInteger (Utilities|Array|LastIndex _spawncoordinate__z_axis_))))) false false)))

(fn ProjectileEnemySpawner
  (bind _spawncoordinate__z_axis_ (Variables|ActorSpawnPosition|GetSpawnCoordinate%20%28Z%20axis%29))
  (bind _availableprojectileenemies (Variables|Objectsspawned|Enemies|GetAvailableProjectileEnemies))
  ;[1 1 1] Projectile Enemy Spawner
  (bind _returnvalue (Game|SpawnActorfromClass (Utilities|Array|Get(acopy) _availableprojectileenemies (Math|Random|RandomInteger (Utilities|Array|Length _availableprojectileenemies))) (Math|Transform|MakeTransform (Transformation|GetWorldLocation (Variables|Default|GetRewardSpawning)) "0, 0, 0" "1,1,1") "Undefined" 0 0))
  ;[1 1 1] Set actor starting position
  (if (Variables|ActorSpawnPosition|GetRandomLocation%20%28Z%20axis%29)
    ;;[0.4588 0.6588 1] Spawn the actor randomly from an array of set coordinates
    (Transformation|SetRelativeLocation (Variables|/Game/EndlessRunner2D/Blueprints/EnemySystem/EnemyActors/ProjectileEnemy/BP_Enemy_Projectile_Main.BP_Enemy_Projectile_Main_C|GetRoot _returnvalue) (Math|Vector|MakeVector (.x (Transformation|GetActorLocation _returnvalue)) (.y (Transformation|GetActorLocation _returnvalue)) (.z (Utilities|Array|Get(acopy) _spawncoordinate__z_axis_ (Math|Random|RandomInteger (Utilities|Array|LastIndex _spawncoordinate__z_axis_))))) false false)))

(fn SpecialEnemySpawner
  (bind _spawncoordinate__z_axis_ (Variables|ActorSpawnPosition|GetSpawnCoordinate%20%28Z%20axis%29))
  (bind _availablespecialenemies (Variables|ObjectsSpawned|Enemies|GetAvailableSpecialEnemies))
  ;[1 1 1] Special Enemy Spawner
  (bind _returnvalue (Game|SpawnActorfromClass (Utilities|Array|Get(acopy) _availablespecialenemies (Math|Random|RandomInteger (Utilities|Array|Length _availablespecialenemies))) (Math|Transform|MakeTransform (Transformation|GetWorldLocation (Variables|Default|GetRewardSpawning)) "0, 0, 0" "1,1,1") "Undefined" 0 0))
  ;[1 1 1] Set actor starting position
  (if (Variables|ActorSpawnPosition|GetRandomLocation%20%28Z%20axis%29)
    ;;[0.4588 0.6588 1] Spawn the actor randomly from an array of set coordinates
    (Transformation|SetRelativeLocation (Variables|/Game/EndlessRunner2D/Blueprints/EnemySystem/EnemyActors/SpecialEnemy/BP_Enemy_Special_Main.BP_Enemy_Special_Main_C|GetRoot _returnvalue) (Math|Vector|MakeVector (.x (Transformation|GetActorLocation _returnvalue)) (.y (Transformation|GetActorLocation _returnvalue)) (.z (Utilities|Array|Get(acopy) _spawncoordinate__z_axis_ (Math|Random|RandomInteger (Utilities|Array|LastIndex _spawncoordinate__z_axis_))))) false false)))