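; Player Paper2D character for the 2D endless runner, handling jump, double jump and run/jump flipbook switching.
; A DoN node counts presses to choose Jump or a Z-override LaunchCharacter, each with its own sound, and resets on landing.
; Flipbooks come from the active character in the GameMode's save game, loaded on character selection and after a tiny BeginPlay delay that lets the GameMode initialise first.
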(event Custom|NewCharacterSelected
  (bind _returnvalue (Game|GetGameMode))
  (bind _sprite (Variables|Default|GetSprite))
  (bind _asbp_game_mode (Utilities|Casting|CastToBP_GameMode _returnvalue))
  (bind _savegameinstance (Variables|/Game/EndlessRunner2D/Blueprints/BP_GameMode.BP_GameMode_C|GetSavegameInstance _asbp_game_mode))
  (bind _asbp_save_game_data (Utilities|Casting|CastToBP_SaveGameData _savegameinstance))
  (bind _activecharacter_save (Variables|/Game/EndlessRunner2D/Blueprints/BP_SaveGameData.BP_SaveGameData_C|GetActiveCharacter_Save _asbp_save_game_data))
  ;[1 1 1] Gets the active selected character from the save game blueprint
  ;;[0.4588 0.6588 1] Store the saved character animations locally for changing the animations states
  (Variables|CharacterSelection|SetSelectedCharacterAnim _activecharacter_save)
  (Sprite|SetFlipbook _sprite (Utilities|Array|Get(acopy) _activecharacter_save))
  (Components|Timeline|SetLooping _sprite true)
  (Components|Timeline|PlayfromStart _sprite))

(event EventOnLanded
  (params (Hit :type Hit%20Result%20Structure%20%28by%20ref%29))
  (bind _sprite (Variables|Default|GetSprite))
  (bind _sprite_2 (Variables|Default|GetSprite))
  ;[1 1 1] Player jump system
  ;;[0.4588 0.6588 1] Player animation switch to run
  (if (Variables|PlayerMovement|GetCanPlayerJump)
    ;;;[0.1333 0.4549 1] Get the Run Animation set for the selected character from the save game file
    (Sprite|SetFlipbook (Variables|Default|GetSprite) (Utilities|Array|Get(acopy) (Variables|CharacterSelection|GetSelectedCharacterAnim)))
    (Components|Timeline|SetLooping _sprite true)
    (Components|Timeline|PlayfromStart _sprite)
    ;;[0.4588 0.6588 1] Set the number of jumps
    (Utilities|FlowControl|DoN (Variables|PlayerMovement|GetNrOfJumps)) ; enters at Reset
  ))

(event EventBeginPlay
  (bind _returnvalue (Game|GetGameMode))
  (bind _sprite (Variables|Default|GetSprite))
  (bind _asbp_game_mode (Utilities|Casting|CastToBP_GameMode _returnvalue))
  (bind _savegameinstance (Variables|/Game/EndlessRunner2D/Blueprints/BP_GameMode.BP_GameMode_C|GetSavegameInstance _asbp_game_mode))
  (bind _asbp_save_game_data (Utilities|Casting|CastToBP_SaveGameData _savegameinstance))
  (bind _activecharacter_save (Variables|/Game/EndlessRunner2D/Blueprints/BP_SaveGameData.BP_SaveGameData_C|GetActiveCharacter_Save _asbp_save_game_data))
  ;[1 1 1] Gets the active selected character from the save game blueprint
  (Utilities|FlowControl|Delay 0.0001) ; Activate event after BP Game Mode Begin event
  ;;[0.4588 0.6588 1] Store the saved character animations locally for changing the animations states
  (Variables|CharacterSelection|SetSelectedCharacterAnim _activecharacter_save)
  (Sprite|SetFlipbook _sprite (Utilities|Array|Get(acopy) _activecharacter_save))
  (Components|Timeline|SetLooping _sprite true)
  (Components|Timeline|PlayfromStart _sprite))

(event Input|ActionEvents|InputActionJump
  (params (Key :type Key%20Structure :default "AnyKey"))
  (bind _sprite (Variables|Default|GetSprite))
  ;[1 1 1] Player jump system
  (:Pressed
    (if (Variables|PlayerMovement|GetCanPlayerJump)
      ;;[0.4588 0.6588 1] Set the number of jumps
      (bind _counter (Utilities|FlowControl|DoN (Variables|PlayerMovement|GetNrOfJumps))
        (:Exit
          (switch int _counter
            (:1
              (Character|Jump) ; First Jump
              (Audio|PlaySound2D "/Game/EndlessRunner2D/SFX/Gameplay/Cue/SC_PlayerJump1.SC_PlayerJump1")
              ;;[0.4588 0.6588 1] Player Jump animation switch
              (Sprite|SetFlipbook _sprite (Utilities|Array|Get(acopy) (Variables|CharacterSelection|GetSelectedCharacterAnim) 1))
              (Components|Timeline|SetLooping _sprite false))
            (:2
              (Character|LaunchCharacter (Variables|PlayerMovement|GetDoubleJumpVelocity) false true) ; Double Jump
              (Audio|PlaySound2D "/Game/EndlessRunner2D/SFX/Gameplay/Cue/SC_PlayerJump2.SC_PlayerJump2")
              (Components|Timeline|PlayfromStart _sprite))))))))

(fn ConstructionScript
  ;[1 1 1] Set the maximum number of jumps
  (Variables|PlayerMovement|SetNrOfJumps 3))