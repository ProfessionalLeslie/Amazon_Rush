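; Base reward pickup for the 2D endless runner that sends its reward amount to the game mode and destroys itself on touching the player's capsule.
; Tick scrolls it along X while movement is enabled and destroys it past a coordinate limit.
; Overlapping the player's coin magnet collision instead detaches it from its holder and interpolates it toward the player at constant speed, as long as the player has health left.
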(event OnComponentBeginOverlap(Collision)
  (params (OverlappedComponent :type Primitive%20Component%20Object%20Reference) (OtherActor :type Actor%20Object%20Reference) (OtherComp :type Primitive%20Component%20Object%20Reference) (OtherBodyIndex :type Integer) (bFromSweep :type Boolean) (SweepResult :type Hit%20Result%20Structure%20%28by%20ref%29))
  (bind _returnvalue (Game|GetPlayerCharacter 0))
  (bind _asch_character_2d (Utilities|Casting|CastToCH_Character2d _returnvalue))
  ;[1 1 1] Reward-Player Collision
  ;;[0.4588 0.6588 1] Check if colided with player
  (Utilities|IsValid _asch_character_2d
    (:Is%20Valid
      (if (== OtherComp (Variables|/Script/Engine.Character|GetCapsuleComponent _asch_character_2d))
        ;;[0.4588 0.6588 1] Set the amount of reward for the player
        (Class|BPIGameModeCommunication|RewardInterface(Message) (Game|GetGameMode) (Variables|Reward|GetRewardAmount))
        (Variables|CoinMagnet|SetIsPlayerInRange false) ; Failsafe for coin magnet powerup
        (Actor|DestroyActor)
        (else
          ;;[0.1333 0.4549 1] If this colision is enabled the reward objects will fly towards the players position (coin magnet powerup)
          (if (== OtherComp (Variables|/Game/EndlessRunner2D/Blueprints/CH_Character2d.CH_Character2d_C|GetCoinMagnetColi _asch_character_2d))
            (Variables|CoinMagnet|SetIsPlayerInRange true)))))))

(event Custom|CoinsMovement
  ;[1 1 1] Coin movement to the player > if coin magnet powerup is active each individual coin goes to the player's position
  (Transformation|DetachFromActor "KeepWorld" "KeepWorld" "KeepWorld") ; Separate the coin from the holder = have separate behaviors
  (Transformation|SetActorRelativeLocation (Math|Interpolation|VInterptoConstant (Transformation|GetActorLocation) (Transformation|GetActorLocation (Game|GetPlayerCharacter 0)) (Utilities|Time|GetWorldDeltaSeconds) (Variables|CoinMagnet|GetCoinMagnetMovementSpeed))))

(event EventTick
  (params (DeltaSeconds :type Float%20%28single-precision%29))
  ;[1 1 1] Actor movement > normal or towards the player if coin magnet powerup is active
  (if (Variables|CoinMagnet|GetIsPlayerInRange)
    ;;[0.4588 0.6588 1] The coins fly to the player only if he is alive
    (if (>= (Variables|/Game/EndlessRunner2D/Blueprints/BP_GameMode.BP_GameMode_C|GetCurrentHealth (.AsBP%20Game%20Mode (Utilities|Casting|CastToBP_GameMode (Game|GetGameMode)))) 1)
      (CallFunction|CoinsMovement) ; If you take coin magnet powerup
      (else
        ;[1 1 1] Actor normal movement - set the speed and direction
        (if (Variables|ActorMovement|GetCanMove) :!label _label
          (Transformation|AddActorWorldOffset (Math|Vector|MakeVector (* DeltaSeconds (Variables|ActorMovement|GetSpeed) (Variables|ActorMovement|GetDirection)) 0.0 0.0))
          ;[1 1 1] Set the maximum coordinates at which the actor gets destroyed
          (if (<= (.x (Transformation|GetActorLocation)) (Variables|ActorMovement|GetDestroyCoordinates))
            (Actor|DestroyActor)))))
    (else
      (goto _label))))

(fn ConstructionScript)