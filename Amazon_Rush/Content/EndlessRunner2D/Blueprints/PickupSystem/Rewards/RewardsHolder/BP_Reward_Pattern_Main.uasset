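; BP_Reward_Pattern_Main is a scrolling reward pattern actor for the 2D endless runner.
; BeginPlay places ObjectHolder at a random height, either within the SpawnCoordinateZ range or at one of its preset points.
; Tick moves the actor along X by speed and direction, destroys it past a limit, and triggers the next spawn once through BP_GameMode when RespawnIndicator crosses a threshold.
; The construction script orients a debug arrow by direction.
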(event EventBeginPlay
  (bind _spawncoordinate_z (Variables|ActorSpawnPosition|GetSpawnCoordinate_Z))
  (bind _objectholder (Variables|Default|GetObjectHolder))
  (bind _spawncoordinate_z_2 (Variables|ActorSpawnPosition|GetSpawnCoordinate_Z))
  ;[1 1 1] Set actor starting position
  (if (Variables|ActorSpawnPosition|GetSetRandomPositionType)
    ;;[1 0.3203 0.4914] Set the random position between a min and a max value
    (Transformation|SetRelativeLocation _objectholder (Math|Vector|MakeVector 0.0 0.0 (Math|Conversions|ToFloat(Integer) (Math|Random|RandomIntegerinRange (Math|Float|Truncate (.z (Utilities|Array|Get(acopy) _spawncoordinate_z))) (Math|Float|Truncate (.z (Utilities|Array|Get(acopy) _spawncoordinate_z (Utilities|Array|LastIndex _spawncoordinate_z))))))) false false)
    (else
      ;;[1 0.8939 0.4913] Set the tandom position between fixed values (determined in the Viewport)
      (Transformation|SetRelativeLocation _objectholder (Utilities|Array|Get(acopy) _spawncoordinate_z_2 (Math|Random|RandomInteger (Utilities|Array|Length _spawncoordinate_z_2))) false false))))

(event EventTick
  (params (DeltaSeconds :type Float%20%28single-precision%29))
  (bind _respawnindicator (Variables|Default|GetRespawnIndicator))
  (bind _returnvalue (Transformation|GetWorldLocation _respawnindicator))
  ;[1 1 1] Actor movement - set the speed and direction
  (Transformation|AddActorWorldOffset (Math|Vector|MakeVector (* DeltaSeconds (Variables|ActorMovement|GetSpeed) (Variables|ActorMovement|GetDirection)) 0.0 0.0))
  ;[1 1 1] Set the maximum coordinates at which the actor gets destroyed
  (if (<= (.x (Transformation|GetActorLocation)) (Variables|ActorMovement|GetDestroyCoordinates))
    (Actor|DestroyActor)
    (elif (or (<= (.x _returnvalue) (Variables|SpawnNextObject|GetSpawnNextObjectCoordinate)) (<= (.x _returnvalue) (Variables|ActorMovement|GetDestroyCoordinates)))
      (Utilities|FlowControl|DoOnce false
        (:Completed
          ;[1 1 1] Triggers the next spawn
          (bind _asbp_game_mode (Utilities|Casting|CastToBP_GameMode (Game|GetGameMode)))
          (Default|BlueprintCom _asbp_game_mode))))))

(fn ConstructionScript
  ;[1 1 1] Set the direction of the arrow in the editor based onthe directio its heading (used for debug)
  (if (< (Variables|ActorMovement|GetDirection) 0.0)
    (Transformation|AddLocalRotation (Variables|Default|GetArrow) (Math|Rotator|MakeRotator 0.0 0.0 0.0) false false)
    (else
      (Transformation|AddLocalRotation (Variables|Default|GetArrow) (Math|Rotator|MakeRotator 0.0 0.0 1.8e+02) false false))))