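; Base power-up actor for a 2D endless runner, scrolling along the X axis.
; While movement is enabled, each Tick offsets it by speed and direction, scaled by delta time for frame-rate independence.
; It destroys itself once its X position drops to or below a set limit; no pickup effect is implemented here.
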(event EventTick
  (params (DeltaSeconds :type Float%20%28single-precision%29))
  ;[1 1 1] Actor movement - set the speed and direction
  (if (Variables|Actormovement|GetCanMove)
    (Transformation|AddActorWorldOffset (Math|Vector|MakeVector (* DeltaSeconds (Variables|Actormovement|GetSpeed) (Variables|ActorMovement|GetDirection)) 0.0 0.0))
    ;[1 1 1] Set the maximum coordinates at which the actor gets destroyed
    (if (<= (.x (Transformation|GetActorLocation)) (Variables|Default|GetActorDestroyCoordinates))
      (Actor|DestroyActor))))

(fn ConstructionScript)