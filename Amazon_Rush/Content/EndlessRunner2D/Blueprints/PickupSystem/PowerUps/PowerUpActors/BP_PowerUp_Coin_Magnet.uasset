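; Coin magnet power-up pickup actor for the 2D endless runner, collected when the player character's capsule overlaps its collision.
; On pickup it sets Magnetism and passes it with MagnetismReset to the game mode through an interface message, leaving the power-up handling to the game mode.
; It then activates the PPickup effect on CH_Character2d and destroys itself.
; The construction script only calls its parent.
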(event OnComponentBeginOverlap(Collision)
  (params (OverlappedComponent :type Primitive%20Component%20Object%20Reference) (OtherActor :type Actor%20Object%20Reference) (OtherComp :type Primitive%20Component%20Object%20Reference) (OtherBodyIndex :type Integer) (bFromSweep :type Boolean) (SweepResult :type Hit%20Result%20Structure%20%28by%20ref%29))
  (bind _returnvalue (Game|GetPlayerCharacter 0))
  ;[1 1 1] Coin magnet Collision
  ;;[0.4588 0.6588 1] Check if colided with player
  (Utilities|IsValid _returnvalue
    (:Is%20Valid
      (if (== OtherComp (Variables|/Script/Engine.Character|GetCapsuleComponent _returnvalue))
        ;;[0.4588 0.6588 1] Triggers and sends reset value to the powerup event in BP_GameMode
        (bind _output_get (Variables|PowerUp|SetMagnetism true))
        (Class|BPIGameModeCommunication|CoinMagnetPowerUpInterface(Message) (Game|GetGameMode) _output_get (Variables|PowerUp|GetMagnetismReset))
        ;;[0.4588 0.6588 1] Activate powerup effect
        (Components|Activation|Activate (Variables|/Game/EndlessRunner2D/Blueprints/CH_Character2d.CH_Character2d_C|GetP_Pickup (.AsCH%20Character%202d (Utilities|Casting|CastToCH_Character2d _returnvalue))) false)
        (Actor|DestroyActor)))))

(fn ConstructionScript
  (|CallParentFunction))