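; Scrolling tile map environment for a 2D endless runner, looping ground, tree and wood sign layers along X with a parallax effect.
; The construction script gathers the tile map components and records their starting positions.
; Each Tick moves every layer by its individual speed, global multiplier and direction, scaled by delta time.
; Layers reaching their own coordinate limit snap back to their starting position.
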(event EventBeginPlay
  ;[1 1 1] Toggles Environment movement
  (if (not (Variables|ParallaxScriptsVariables|GetEnvironmentLoop))
    (Variables|ParallaxScriptsVariables|SetEnvironmentLoop true)))

(event EventTick
  (params (DeltaSeconds :type Float%20%28single-precision%29))
  (Variables|ParallaxScriptsVariables|SetTheTime DeltaSeconds)
  (if (Variables|ParallaxScriptsVariables|GetEnvironmentLoop)
    ;[1 1 1] Environment elements individual movement
    ;;[0.4588 0.6588 1] Gets one element at a time
    (for (_array_element _array_index) (Variables|ParallaxScriptsVariables|GetMainObjectsHolder)
      (Variables|ParallaxScriptsVariables|SetCurrentObjectIndex _array_index)
      ;;[0.4588 0.6588 1] Resets to original position
      (if (or (Math|Float|NearlyEqual(Float) (* (.X (Math|Vector|BreakVector (Variables|/Script/Engine.SceneComponent|GetRelativeLocation _array_element))) (Variables|ParallaxScriptsVariables|GetDirectionDetection)) (.X (Math|Vector|BreakVector (Utilities|Array|Get(acopy) (Variables|ChangeFirst|GetObjectMaxCoordLimit) (Variables|ParallaxScriptsVariables|GetCurrentObjectIndex)))) 1.0) (>= (* (.X (Math|Vector|BreakVector (Variables|/Script/Engine.SceneComponent|GetRelativeLocation _array_element))) (Variables|ParallaxScriptsVariables|GetDirectionDetection)) (.X (Math|Vector|BreakVector (Utilities|Array|Get(acopy) (Variables|ChangeFirst|GetObjectMaxCoordLimit) (Variables|ParallaxScriptsVariables|GetCurrentObjectIndex))))))
        (Transformation|SetRelativeLocation _array_element (Utilities|Array|Get(acopy) (Variables|ParallaxScriptsVariables|GetInitialPosition) (Variables|ParallaxScriptsVariables|GetCurrentObjectIndex)) false false)
        (else
          ;;[0.4588 0.6588 1] Sends the chosen element in a direction at a certain speed (parallax)
          (Transformation|AddRelativeLocation _array_element (Math|Vector|MakeVector (* (* (* (Utilities|Array|Get(acopy) (Variables|ChangeFirst|GetObjectIndividualSpeed) _array_index) (Variables|ParallaxScriptsVariables|GetTheTime)) (Variables|ParallaxScriptsVariables|GetSpeedMultiplier)) (Variables|ParallaxScriptsVariables|GetDirectionDetection)) 0.0 0.0) false false))))))

(fn ConstructionScript
  ;[1 1 1] The environment elements holder
  (bind _output_get (Variables|ParallaxScriptsVariables|SetMainObjectsHolder (Utilities|Array|MakeArray (Variables|Default|GetTM_Ground) (Variables|Default|GetTM_Trees1) (Variables|Default|GetTM_WoodSigns) (Variables|Default|GetTM_Trees2))))
  (for _array_element _output_get
    ;[1 1 1] Get the initial position of each element
    (Utilities|Array|Add (Variables|ParallaxScriptsVariables|GetInitialPosition) (Variables|/Script/Engine.SceneComponent|GetRelativeLocation _array_element))))